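; Main menu game mode that puts the OGT main menu widget on screen when play starts.
; On BeginPlay it shows the mouse cursor, creates WB_OGTMainMenu and adds it to the viewport.
; It then sets input mode to game only despite the menu being shown.
; An else branch would remove the widget if it were already in the viewport.
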(event EventBeginPlay
  ;[0.5 1 1] Show Main Menu after start play
  (Variables|/Script/Engine.PlayerController|SetbShowMouseCursor (Game|GetPlayerController 0) true)
  (bind _returnvalue (UserInterface|CreateWidget "/Game/UI/MainMenu/WB_OGTMainMenu.WB_OGTMainMenu_C"))
  (Variables|Default|SetMainMenuWidget _returnvalue)
  (if (not (UserInterface|Viewport|IsinViewport (Variables|Default|GetMainMenuWidget)))
    (UserInterface|Viewport|AddtoViewport (Variables|Default|GetMainMenuWidget) 0)
    (Input|SetInputModeGameOnly (Game|GetPlayerController 0) false)
    (else
      (Widget|RemovefromParent (Variables|Default|GetMainMenuWidget)))))

(fn ConstructionScript)
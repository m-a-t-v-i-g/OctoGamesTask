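; BP_Trigger_Door1 is an interactable door that swings open and closed around its yaw axis.
; CallInteract flips the Closed flag and sets the target yaw to either an open angle or zero.
; Every Tick, UpdateRotation eases the static mesh's relative yaw toward that target with FInterpTo, giving a smooth swing without a Timeline.
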(event EventTick
  (params (DeltaSeconds :type Float%20%28single-precision%29))
  (CallFunction|UpdateRotation DeltaSeconds))

(event EventCallInteract
  (if (Variables|Default|GetClosed)
    (Variables|Default|SetSetRotation 1.2e+02)
    (Variables|Default|SetClosed false)
    (else
      (Variables|Default|SetSetRotation 0.0)
      (Variables|Default|SetClosed true))))

(fn ConstructionScript)

(fn UpdateRotation
  (params (DeltaTime :type Float%20%28double-precision%29))
  (Transformation|SetRelativeRotation (Variables|Default|GetStaticMeshComponent) (Math|Rotator|MakeRotator 0.0 0.0 (Math|Interpolation|FInterpTo (.yaw (Variables|/Script/Engine.SceneComponent|GetRelativeRotation (Variables|Default|GetStaticMeshComponent))) (Variables|Default|GetSetRotation) DeltaTime 5.0)) false false))